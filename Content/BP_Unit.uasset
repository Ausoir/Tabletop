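; BP_Unit is a grid-based unit Actor that moves through a voxel world on a turn-delay cooldown.
; A looping timer counts down TurnDelay and drops the unit into clear voxels below, acting as gravity.
; Move spends the delay through CostTurn, then tries the horizontal direction, falling back to stepping up when blocked.
; Logic changes only the integer Coord, while Tick lerps the actor toward it for smooth motion.
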(event `self.ReceiveBeginPlay`
  (`KismetSystemLibrary.K2_SetTimer` null "ProcessTurn" 0.1 true)
  (`self.ReadjustCoord`))

(event `self.ReceiveTick`
  (params (DeltaSeconds :type "Float (single-precision)"))
  (bind _vec (`/Game/FunctionLibrary.CoordToVec` (`self.Coord`)))
  (`self.K2_SetActorLocation` (`KismetMathLibrary.VLerp` (`self.K2_GetActorLocation`) _vec 0.1)))

(fn `Move`
  (params (Cost :type Integer) (Direction :type Integer) (Climb :type Boolean))
  (locals (Left :type "IntVector Structure" :default (struct :`Y` -1)) (Up :type "IntVector Structure" :default (struct :`X` 1)) (Right :type "IntVector Structure" :default (struct :`Y` 1)) (Down :type "IntVector Structure" :default (struct :`X` -1)) (Dir :type "IntVector Structure"))
  (`self.CostTurn` Cost
    (:`Success`
      (set `local.Dir` (select `int` Direction :`0` (struct) :`1` (`local.Left`) :`2` (`local.Up`) :`3` (`local.Right`) :`4` (`local.Down`) :`5` (struct)))
      (bind (_found _dest) (`/Game/FunctionLibrary.IsVoxelClearTo` (`self.Coord`) (`local.Dir`) 55.0))
      (if _found
        (set `self.Coord` _dest)
        (else
          (bind (_found_2 _dest_2) (`/Game/FunctionLibrary.IsVoxelClearTo` (`self.Coord`) (make `IntVector` 0 0 1) 25.0))
          (if _found_2
            (bind (_found_3 _dest_3) (`/Game/FunctionLibrary.IsVoxelClearTo` _dest_2 (`local.Dir`) 55.0))
            (if _found_3
              (set `self.Coord` _dest_3)
              (else
                (bind (_found_4 _dest_4) (`/Game/FunctionLibrary.IsVoxelClearTo` _dest_2 (+ (`local.Dir`) (make `IntVector` 0 0 1)) 60.0))
                (if _found_4
                  (set `self.Coord` _dest_4))))))))))

(fn `MoveBelow`
  (bind (_found _dest) (`/Game/FunctionLibrary.IsVoxelClearTo` (`self.Coord`) (make `IntVector` 0 0 -1) 30.0))
  (if _found
    (set `self.Coord` _dest)))

(fn `ProcessTurn`
  (bind _result (`/Engine/EditorBlueprintResources/StandardMacros.DecrementInt` (`self.TurnDelay`))
    (:`  `
      (set `self.TurnDelay` (`KismetMathLibrary.Max` _result))
      (`self.MoveBelow`))))

(fn `ReadjustCoord`
  (bind _newparam (`/Game/FunctionLibrary.VecToCoord` (`self.K2_GetActorLocation`)))
  (set `self.Coord` _newparam))

(fn `UserConstructionScript`
  (`PrimitiveComponent.SetMaterial` (`self.Plane`) 0 (`self.Material`)))