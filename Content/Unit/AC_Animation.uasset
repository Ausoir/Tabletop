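; Unit animation component that plays keyframed motion from the AnimationList data table on a Plane component.
; SetAnimation loads a row by name and restarts the index; Tick then applies one translation, rotation and scale entry per frame until translations run out, independent of delta time.
; SetDir converts a grid direction into an angle that rotates each translation about the Y axis, while rotation entries drive yaw only.
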(event `self.ReceiveTick`
  (params (DeltaSeconds :type "Float (single-precision)"))
  (bind _currentindex (`self.CurrentIndex`))
  (bind (_translation _rotation _scale) (break `/Game/Structure/St_AnimationValues` (`self.Values`)))
  (if (< (`self.CurrentIndex`) (`KismetArrayLibrary.Array_Length` _translation))
    (`self.TickTransform` (`|GetArrayItem` _translation _currentindex) (`|GetArrayItem` _rotation _currentindex) (`|GetArrayItem` _scale _currentindex))
    (bind _result (`/Engine/EditorBlueprintResources/StandardMacros.IncrementInt` (`self.CurrentIndex`))
      (:`  `
        (set `self.CurrentIndex` _result)))))

(fn `SetAnimation`
  (params (AnimName :type Name))
  (bind _returnvalue (`|GetDataTableRow` "/Game/Structure/AnimationList.AnimationList" AnimName)
    (:`then`
      (set `self.Values` _returnvalue)
      (set `self.CurrentIndex` 0))))

(fn `SetDir`
  (params (Dir :type "IntVector Structure"))
  (bind (_x _y) (break `IntVector` Dir))
  (switch `int` _x
    (:`Default`
      (set `self.Dir` 180.0))
    (:`0`
      (switch `int` _y
        (:`Default`
          (set `self.Dir` 90.0))
        (:`1`
          (set `self.Dir` -90.0))))
    (:`1`
      (set `self.Dir` 0.0))))

(fn `TickTransform`
  (params (Value :type "Vector Structure") (Rotation :type "Float (double-precision)") (Scale :type "Vector Structure"))
  (`SceneComponent.K2_SetRelativeTransform` (`self.Plane`) (`KismetMathLibrary.MakeTransform` (`KismetMathLibrary.RotateAngleAxis` Value (`self.Dir`) (0.0 1.0 0.0)) (`KismetMathLibrary.MakeRotator` 0.0 0.0 Rotation) Scale) false false))