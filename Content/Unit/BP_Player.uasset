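; BP_Player is the player unit that moves by direction while exploring and fights turn-based card battles when engaged.
; AI perception engages live foes, numbers them for turn order and counts their deaths.
; Engaged direction input plays the next hand card from a data table on that direction's distance-sorted target list.
; Four cards end the turn and dispatch to foes, while victory or defeat clears combat state.
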(event `self.ReceiveBeginPlay`
  (`parent.ReceiveBeginPlay`)
  (bind _playercontrol (`/Game/Game/FunctionLibrary.GetController`))
  (add `/Game/Game/BP_Controller.DispatchMovement` _playercontrol (delegate `DispatchMovement_Event`)))

(event `DispatchMovement_Event`
  (params (Dir :type Integer))
  (if (`self.Engaged`)
    (`self.FaceDir` Dir)
    (`KismetSystemLibrary.Delay` 0.3)
    (`self.AttackDirection` Dir
      (:`TurnEnd`
        (`self.EndTurn`)))
    (else
      (`self.Move` 3 Dir true))))

(event `self.AIPerception.OnTargetPerceptionUpdated`
  (params (Actor :type "Actor Object Reference") (Stimulus :type "AIStimulus Structure"))
  (bind _index (`self.Index`))
  (bind _asbp_foe (cast `/Game/Unit/BP_Foe` Actor))
  (if (not (`/Game/Unit/BP_Unit.Dead` _asbp_foe))
    (`self.Engage` _asbp_foe true)
    (`/Game/Unit/BP_Foe.SetArrow` _asbp_foe (`self.K2_GetActorLocation`))
    (`self.Event SetIndex` _asbp_foe _index)
    (bind _result (`/Engine/EditorBlueprintResources/StandardMacros.IncrementInt` _index)
      (:`  `
        (set `self.Index` _result)
        (`self.Engage` true)
        (add `self.DispatchOnDead` _asbp_foe (delegate `DispatchOnDead_Event`))
        (add `self.DispatchTurns` (delegate `self.DispatchTurn_Event`))
        (`KismetSystemLibrary.Delay` 0.3)
        (bind _playercontrol (`/Game/Game/FunctionLibrary.GetController`))
        (`self.EnableInput` _playercontrol _playercontrol)))))

(event `self.DispatchTurn_Event`
  (params (Index :type Integer))
  (if (== Index (`self.Index`))
    (bind _result (`self.CheckGameState`))
    (switch `int` _result
      (:`0`
        (`self.Turn` false)))))

(event `DispatchOnDead_Event` :!signature `self.DispatchOnDead`
  (params (UIndex :type Integer))
  (bind _result (`/Engine/EditorBlueprintResources/StandardMacros.IncrementInt` (`self.DeadFoes`))
    (:`  `
      (set `self.DeadFoes` _result))))

(event `EndTurn`
  (`self.DispatchEnd`)
  (bind _playercontrol (`/Game/Game/FunctionLibrary.GetController`))
  (`self.DisableInput` _playercontrol _playercontrol)
  (`KismetSystemLibrary.Delay` 0.3)
  (`self.DispatchTurns` 0))

(fn `AddArrow`
  (params (Index :type Integer) (Unit :type "/Game/Unit/BP_Unit Object Reference"))
  (switch `int` Index
    (:`0`
      (`self.AddToArrow` (`self.ArrowLeft`) Unit))
    (:`1`
      (`self.AddToArrow` (`self.ArrowUp`) Unit))
    (:`2`
      (`self.AddToArrow` (`self.ArrowRight`) Unit))
    (:`3`
      (`self.AddToArrow` (`self.ArrowDown`) Unit))))

(fn `AddToArrow`
  (params (List :type "Array of /Game/Unit/BP_Unit Object Reference") (Adding :type "/Game/Unit/BP_Unit Object Reference"))
  (for (_array_element _array_index) List
    (if (< (`self.GetDistanceTo` Adding) (`self.GetDistanceTo` _array_element))
      (`KismetArrayLibrary.Array_Insert` List Adding _array_index)
      (return)))
  (`KismetArrayLibrary.Array_Add` List Adding)
  (return))

(fn `CheckGameState`
  (returns (Result :type Integer))
  (locals (State :type Integer))
  (`|ExecutionSequence`
    (:`then_0`
      (if (>= (`self.DeadFoes`) (`self.Index`))
        (set `local.State` 1)
        (`self.Engage` false :!label _label)
        (`KismetArrayLibrary.Array_Clear` (`self.ArrowLeft`))
        (`KismetArrayLibrary.Array_Clear` (`self.ArrowUp`))
        (`KismetArrayLibrary.Array_Clear` (`self.ArrowRight`))
        (`KismetArrayLibrary.Array_Clear` (`self.ArrowDown`))
        (set `self.DeadFoes` 0)
        (set `self.Index` 0)))
    (:`then_1`
      (if (`self.Dead`)
        (set `local.State` 2)
        (goto _label)))
    (:`then_2`
      (return (`local.State`)))))

(fn `Engage`
  (params (Engage :type Boolean))
  (`|ExecutionSequence`
    (:`then_0`
      (if Engage
        (if (not (`self.Engaged`))
          (`self.DispatchEngage`)
          (bind _playercontrol (`/Game/Game/FunctionLibrary.GetController`))
          (`self.DisableInput` _playercontrol _playercontrol))
        (else
          (`self.DispatchEnd`)
          (bind _playercontrol_2 (`/Game/Game/FunctionLibrary.GetController`))
          (`self.EnableInput` _playercontrol_2 null))))
    (:`then_1`
      (`parent.Engage` Engage)
      (set `self.Hand` 0))))

(fn `PlayHand`
  (params (Index :type Integer) (On :type "Array of /Game/Unit/BP_Unit Object Reference"))
  (bind _asbp_controller (cast `/Game/Game/BP_Controller` (`self.GetController`)))
  (bind _card (`/Game/Game/BP_Controller.FetchHand` _asbp_controller Index))
  (bind _returnvalue (`|GetDataTableRow` "/Game/Structure/CardList.CardList" _card)
    (:`then`
      (`self.UseCard` _returnvalue On)
      (`self.DispatchUse` Index))))

(fn `Turn`
  (params (Skip :type Boolean))
  (bind _playercontrol (`/Game/Game/FunctionLibrary.GetController`))
  (`self.EnableInput` _playercontrol _playercontrol)
  (`/Game/Game/BP_Controller.ShuffleHand` _playercontrol)
  (`self.DispatchEngage`)
  (set `self.Hand` 0))

(fn `UserConstructionScript`
  (`parent.UserConstructionScript`))