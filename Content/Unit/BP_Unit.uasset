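; BP_Unit is a grid-based unit with health, block and card effects, shown on a plane with stat displays.
; A timer refills turn points for moves, which can climb one step; Tick lerps the actor to its coord and drops it when unsupported.
; Engaging pauses that timer, while indexed turns chain through the player's dispatcher.
; UseCard applies buffs to itself and afflictions to targets via ACUnit, then refreshes display and death state.
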(event `self.ReceiveBeginPlay`
  (`KismetSystemLibrary.K2_SetTimer` null "ProcessTurn" 0.1 true)
  (`self.ReadjustCoord`)
  (`self.Refresh`))

(event `self.ReceiveTick`
  (params (DeltaSeconds :type "Float (single-precision)"))
  (`self.MoveBelow`)
  (bind _vec (`/Game/Game/FunctionLibrary.CoordToVec` (`self.Coord`)))
  (`self.K2_SetActorLocation` (`KismetMathLibrary.VLerp` (`self.K2_GetActorLocation`) _vec 0.1)))

(event `Event SetIndex`
  (params (Index :type Integer))
  (set `self.Index` Index)
  (bind _newparam (`/Game/Game/FunctionLibrary.GetPlayer`))
  (add `/Game/Unit/BP_Player.DispatchTurns` _newparam (delegate `DispatchTurn_Event`)))

(event `DispatchTurn_Event`
  (params (Index :type Integer))
  (if (== Index (`self.Index`))
    (bind _newparam (`/Game/Unit/AC_Unit.IsDead` (`self.AC_Unit`)))
    (if _newparam
      (`self.Turn` true)
      (else
        (`KismetSystemLibrary.Delay` 0.2)
        (`self.Turn` false)))))

(fn `Die`
  (if (not (`self.Dead`))
    (set `self.Dead` true)
    (`SceneComponent.SetHiddenInGame` (`self.HealthPlane`) true true)
    (`SceneComponent.K2_SetRelativeLocationAndRotation` (`self.ModelRoot`) (0.0 0.0 -10.0) (struct :`Yaw` 45.0) false false)
    (`self.DispatchOnDead` (`self.Index`))))

(fn `Engage`
  (params (Engage :type Boolean))
  (bind _output_get (set `self.Engaged` Engage))
  (if _output_get
    (`KismetSystemLibrary.K2_PauseTimer` null "ProcessTurn")
    (else
      (`KismetSystemLibrary.K2_UnPauseTimer` null "ProcessTurn"))))

(fn `FaceDir`
  (params (Dir :type Integer))
  (locals (Left :type "IntVector Structure" :default (struct :`X` -1)) (Up :type "IntVector Structure" :default (struct :`Y` -1)) (Right :type "IntVector Structure" :default (struct :`X` 1)) (Down :type "IntVector Structure" :default (struct :`Y` 1)))
  (bind _output_get (set `self.LastDir` (select `int` Dir :`0` (`local.Left`) :`1` (`local.Up`) :`2` (`local.Right`) :`3` (`local.Down`))))
  (`/Game/Unit/AC_Animation.SetDir` (`self.AC_Animation`) _output_get))

(fn `Move`
  (params (Cost :type Integer) (Direction :type Integer) (Climb :type Boolean))
  (locals (Left :type "IntVector Structure" :default (struct :`X` -1)) (Up :type "IntVector Structure" :default (struct :`Y` -1)) (Right :type "IntVector Structure" :default (struct :`X` 1)) (Down :type "IntVector Structure" :default (struct :`Y` 1)))
  (`self.CostTurn` Cost
    (:`Success`
      (`self.FaceDir` Direction)
      (`/Game/Unit/AC_Animation.SetAnimation` (`self.AC_Animation`) "Move")
      (bind (_collision _dest) (`/Game/Game/FunctionLibrary.IsLineClearTo` (`self.Coord`) (`self.LastDir`) 1))
      (if _collision
        (set `self.Coord` _dest)
        (else
          (bind (_collision_2 _dest_2) (`/Game/Game/FunctionLibrary.IsLineClearTo` (`self.Coord`) (make `IntVector` 0 0 1) 1))
          (if _collision_2
            (bind (_collision_3 _dest_3) (`/Game/Game/FunctionLibrary.IsLineClearTo` _dest_2 (`self.LastDir`) 1))
            (if _collision_3
              (set `self.Coord` _dest_3))))))))

(fn `MoveBelow`
  (bind (_collision _dest) (`/Game/Game/FunctionLibrary.IsLineClearTo` (`self.Coord`) (make `IntVector` 0 0 -1) 1))
  (if _collision
    (set `self.Coord` _dest)))

(fn `MoveToward`
  (params (Dest :type "Vector Structure"))
  (bind _x (.x (- Dest (`self.K2_GetActorLocation`))))
  (bind _y (.y (- Dest (`self.K2_GetActorLocation`))))
  (if (> (`KismetMathLibrary.Abs` _x) (`KismetMathLibrary.Abs` _y))
    (if (> _x 0.0)
      (`self.Move` 3 2 true)
      (else
        (`self.Move` 3 0 true)))
    (elif (> _y 0.0)
      (`self.Move` 3 3 true)
      (else
        (`self.Move` 3 1 true)))))

(fn `ProcessTurn`
  (set `self.TurnPoints` (`KismetMathLibrary.Min` (+ (`self.TurnPoints`) 2) 3)))

(fn `ReadjustCoord`
  (bind _newparam (`/Game/Game/FunctionLibrary.VecToCoord` (`self.K2_GetActorLocation`)))
  (set `self.Coord` _newparam))

(fn `Refresh`
  (bind _block (`/Game/Unit/AC_Unit.Block` (`self.AC_Unit`)))
  (bind _newparam (`/Game/Unit/AC_Unit.IsDead` (`self.AC_Unit`)))
  (if _newparam
    (`self.Die`)
    (`SceneComponent.SetHiddenInGame` (`self.Scene`) true true)
    (else
      (`TextRenderComponent.K2_SetText` (`self.TextRender`) (`KismetTextLibrary.Conv_IntToText` (`/Game/Unit/AC_Unit.Health` (`self.AC_Unit`))))
      (`SceneComponent.SetHiddenInGame` (`self.ShieldPlane`) (== _block 0) true)
      (`TextRenderComponent.K2_SetText` (`self.TextShield`) (`KismetTextLibrary.Conv_IntToText` _block)))))

(fn `Turn`
  (params (Skip :type Boolean))
  (bind _newparam (`/Game/Game/FunctionLibrary.GetPlayer`))
  (`/Game/Unit/BP_Player.DispatchTurns` _newparam (+ (`self.Index`) 1)))

(fn `UseBuff`
  (params (Level :type Integer) (Buffs :type "Array of Name"))
  (for _array_element Buffs
    (`/Game/Unit/AC_Unit.ApplyEffect` (`self.AC_Unit`) _array_element Level))
  (`self.Refresh`))

(fn `UseCard`
  (params (Card :type "/Game/Structure/St_Card Structure") (On :type "Array of /Game/Unit/BP_Unit Object Reference"))
  (bind (_name _image _level _buff _afflict) (break `/Game/Structure/St_Card` Card))
  (`|ExecutionSequence`
    (:`then_0`
      (if (`KismetArrayLibrary.Array_IsNotEmpty` _buff)
        (`self.UseBuff` _level _buff)
        (`/Game/Unit/AC_Animation.SetAnimation` (`self.AC_Animation`) "Eat")))
    (:`then_1`
      (if (`KismetArrayLibrary.Array_IsNotEmpty` _afflict)
        (for _array_element On
          (`self.UseBuff` _array_element _level _afflict))
        (`/Game/Unit/AC_Animation.SetAnimation` (`self.AC_Animation`) "Attack")))))

(fn `UserConstructionScript`
  (`PrimitiveComponent.SetMaterial` (`self.Plane`) 0 (`self.Material`))
  (set `/Game/Unit/AC_Animation.Plane` (`self.Plane`) (`self.AC_Animation`)))