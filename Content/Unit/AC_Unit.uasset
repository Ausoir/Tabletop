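; AC_Unit is a unit component that tracks Health, Block and Mana and applies leveled effects to them.
; ApplyEffect routes Damage, Heal, Block and Mana effects, granting Block through negative damage.
; Damage consumes Block, but zeroes it before subtracting from Health, so breaking hits land in full.
; "Hit" plays through BP_Unit's ACAnimation when Damage returns false: fully blocked or Health depleted.
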(fn `ApplyEffect`
  (params (Effect :type Name) (Level :type Integer))
  (switch `name` Effect
    (:`Damage`
      (bind _dead (`self.Damage` Level))
      (if (not _dead)
        (`self.SetAnimation` "Hit")))
    (:`Heal`
      (`self.Heal` Level))
    (:`Block`
      (`self.Damage` (* Level -1)))
    (:`Mana`
      (`self.ManaGain` Level))))

(fn `Damage`
  (params (Damage :type Integer))
  (returns (Dead :type Boolean))
  (bind _returnvalue (- (`self.Block`) Damage))
  (if (> _returnvalue 0)
    (set `self.Block` _returnvalue)
    (return false)
    (else
      (set `self.Block` 0)
      (bind _output_get (set `self.Health` (+ _returnvalue (`self.Health`))))
      (return (> _output_get 0)))))

(fn `Heal`
  (params (Heal :type Integer))
  (set `self.Health` (+ Heal (`self.Health`))))

(fn `IsDead`
  (returns (NewParam :type Boolean))
  (return (<= (`self.Health`) 0)))

(fn `ManaGain`
  (params (Gain :type Integer))
  (set `self.Mana` (+ Gain (`self.Mana`))))

(fn `SetAnimation`
  (params (Animation :type Name))
  (bind _asbp_unit (cast `/Game/Unit/BP_Unit` (`self.GetOwner`)))
  (`/Game/Unit/AC_Animation.SetAnimation` (`/Game/Unit/BP_Unit.AC_Animation` _asbp_unit) Animation))