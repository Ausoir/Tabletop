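; BP_Foe is a foe unit that can display a directional arrow and register it with the player.
; SetArrow reveals Plane2 and converts the vector from a given point to the foe into a cardinal index.
; It passes that index and itself to the player's AddArrow, then moves the plane to a preset relative transform for that direction.
; The event graph holds only disabled default events.
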(fn `SetArrow`
  (params (From :type "Vector Structure"))
  (bind _plane2 (`self.Plane2`))
  (`SceneComponent.SetHiddenInGame` (`self.Plane2`) false false)
  (bind _direction (`/Game/Game/FunctionLibrary.VectorToCardinal` (- (`self.K2_GetActorLocation`) From)))
  (bind _newparam (`/Game/Game/FunctionLibrary.GetPlayer`))
  (`/Game/Unit/BP_Player.AddArrow` _newparam _direction self)
  (switch `int` _direction
    (:`0`
      (`SceneComponent.K2_SetRelativeLocationAndRotation` _plane2 (15.0 10.0 -10.0) (struct :`Yaw` -90.0) false false))
    (:`1`
      (`SceneComponent.K2_SetRelativeLocationAndRotation` :`self` _plane2 :`NewLocation` (0.0 20.0 -10.0)))
    (:`2`
      (`SceneComponent.K2_SetRelativeLocationAndRotation` _plane2 (-15.0 10.0 -10.0) (struct :`Yaw` 90.0) false false))
    (:`3`
      (`SceneComponent.K2_SetRelativeLocationAndRotation` _plane2 (0.0 10.0 -10.0) (struct :`Yaw` 180.0) false false))))

(fn `UserConstructionScript`
  (`parent.UserConstructionScript`))