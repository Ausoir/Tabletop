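; AI controller for BP_Unit pawns that chases the player, spending turns gated by the unit's TurnPoints.
; A perception update on a BP_Player stores it as the target and enables Tick, which requests a path whenever TurnPoints exceeds a threshold.
; PathToTarget runs a synchronous navmesh query from the controller's own location and passes only the second path point to the unit's MoveToward, printing the length if the path is empty.
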(event `self.ReceiveTick`
  (params (DeltaSeconds :type "Float (single-precision)"))
  (bind _asbp_unit (cast `/Game/Unit/BP_Unit` (`self.K2_GetPawn`)))
  (if (> (`/Game/Unit/BP_Unit.TurnPoints` _asbp_unit) 2)
    (`self.PathToTarget`)))

(event `self.AIPerception.OnTargetPerceptionUpdated`
  (params (Actor :type "Actor Object Reference") (Stimulus :type "AIStimulus Structure"))
  (bind _asbp_player (cast `/Game/Unit/BP_Player` Actor))
  (set `self.Target` _asbp_player)
  (`self.SetActorTickEnabled` true))

(fn `PathToTarget`
  (bind _returnvalue (`NavigationSystemV1.FindPathToLocationSynchronously` (`self.K2_GetActorLocation`) (`self.K2_GetActorLocation` (`self.Target`)) (`self.NavMesh`) "/Script/NavigationSystem.RecastFilter_UseDefaultArea"))
  (bind _pathpoints (`NavigationPath.PathPoints` _returnvalue))
  (if (`KismetArrayLibrary.Array_IsNotEmpty` _pathpoints)
    (bind _asbp_unit (cast `/Game/Unit/BP_Unit` (`self.K2_GetPawn`)))
    (`/Game/Unit/BP_Unit.MoveToward` _asbp_unit (`|GetArrayItem` _pathpoints 1))
    (else
      (`KismetSystemLibrary.PrintString` (`KismetStringLibrary.Conv_IntToString` (`KismetArrayLibrary.Array_Length` _pathpoints))))))

(fn `UserConstructionScript`
  (bind _returnvalue (`GameplayStatics.GetActorOfClass` "/Script/NavigationSystem.NavMeshBoundsVolume"))
  (set `self.NavMesh` _returnvalue))