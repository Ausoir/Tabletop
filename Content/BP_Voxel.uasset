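; BP_Voxel is a voxel world Blueprint that stamps a test data asset into the terrain once the world has loaded.
; BeginPlay calls the parent and binds the world-loaded event, which imports the Test asset at a fixed offset, merging all values and materials.
; An unconnected graph fragment parses string rows character by character, adding a voxel box wherever an X appears, like an ASCII-map builder.
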(event `self.ReceiveBeginPlay`
  (`parent.ReceiveBeginPlay`)
  (add `self.OnWorldLoaded` (delegate `OnWorldLoaded_Event`)))

(event `OnWorldLoaded_Event`
  (`VoxelAssetTools.ImportDataAssetFast` null "/Game/test.test" (-100.0 -100.0 50.0) "AllValuesAndAllMaterials"))

(fn `UserConstructionScript`)