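; BP_Controller turns Enhanced Input actions into event dispatcher broadcasts for four hands and four movement directions.
; BeginPlay adds the IMC mapping context, and the directional actions broadcast an index through the Movement dispatcher.
; Each number action shuffles its hand array before broadcasting that index through the Numkey dispatcher.
; FetchHand returns the first element of an indexed hand, and ShuffleHand reshuffles all four.
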(event `self.ReceiveBeginPlay`
  (`EnhancedInputSubsystemInterface.AddMappingContext` (pcsubsystem `EnhancedInputLocalPlayerSubsystem` (`GameplayStatics.GetPlayerController` 0)) "/Game/Input/IMC.IMC" 0 (struct)))

(event `EnhancedInput|/Game/Input/IA_1`
  (params (ActionValue :type "Float (double-precision)") (ElapsedSeconds :type "Float (double-precision)") (TriggeredSeconds :type "Float (double-precision)") (InputAction :type "InputAction Object Reference" :default "/Game/Input/IA_1.IA_1"))
  (:`Started`
    (`KismetArrayLibrary.Array_Shuffle` (`self.Hand_0`))
    (`self.DispatchNumkey` 0)))

(event `EnhancedInput|/Game/Input/IA_Left`
  (params (ActionValue :type Boolean) (ElapsedSeconds :type "Float (double-precision)") (TriggeredSeconds :type "Float (double-precision)") (InputAction :type "InputAction Object Reference" :default "/Game/Input/IA_Left.IA_Left"))
  (:`Triggered`
    (`self.DispatchMovement` 0)))

(event `EnhancedInput|/Game/Input/IA_Up`
  (params (ActionValue :type Boolean) (ElapsedSeconds :type "Float (double-precision)") (TriggeredSeconds :type "Float (double-precision)") (InputAction :type "InputAction Object Reference" :default "/Game/Input/IA_Up.IA_Up"))
  (:`Triggered`
    (`self.DispatchMovement` 1)))

(event `EnhancedInput|/Game/Input/IA_2`
  (params (ActionValue :type "Float (double-precision)") (ElapsedSeconds :type "Float (double-precision)") (TriggeredSeconds :type "Float (double-precision)") (InputAction :type "InputAction Object Reference" :default "/Game/Input/IA_2.IA_2"))
  (:`Started`
    (`KismetArrayLibrary.Array_Shuffle` (`self.Hand_1`))
    (`self.DispatchNumkey` 1)))

(event `EnhancedInput|/Game/Input/IA_Right`
  (params (ActionValue :type Boolean) (ElapsedSeconds :type "Float (double-precision)") (TriggeredSeconds :type "Float (double-precision)") (InputAction :type "InputAction Object Reference" :default "/Game/Input/IA_Right.IA_Right"))
  (:`Triggered`
    (`self.DispatchMovement` 2)))

(event `EnhancedInput|/Game/Input/IA_3`
  (params (ActionValue :type "Float (double-precision)") (ElapsedSeconds :type "Float (double-precision)") (TriggeredSeconds :type "Float (double-precision)") (InputAction :type "InputAction Object Reference" :default "/Game/Input/IA_3.IA_3"))
  (:`Started`
    (`KismetArrayLibrary.Array_Shuffle` (`self.Hand_2`))
    (`self.DispatchNumkey` 2)))

(event `EnhancedInput|/Game/Input/IA_Down`
  (params (ActionValue :type Boolean) (ElapsedSeconds :type "Float (double-precision)") (TriggeredSeconds :type "Float (double-precision)") (InputAction :type "InputAction Object Reference" :default "/Game/Input/IA_Down.IA_Down"))
  (:`Triggered`
    (`self.DispatchMovement` 3)))

(event `EnhancedInput|/Game/Input/IA_4`
  (params (ActionValue :type "Float (double-precision)") (ElapsedSeconds :type "Float (double-precision)") (TriggeredSeconds :type "Float (double-precision)") (InputAction :type "InputAction Object Reference" :default "/Game/Input/IA_4.IA_4"))
  (:`Started`
    (`KismetArrayLibrary.Array_Shuffle` (`self.Hand_3`))
    (`self.DispatchNumkey` 3)))

(fn `FetchHand`
  (params (Index :type Integer))
  (returns (Card :type Name))
  (switch `int` Index
    (:`0`
      (return (`|GetArrayItem` (`self.Hand_0`))))
    (:`1`
      (return (`|GetArrayItem` (`self.Hand_1`))))
    (:`2`
      (return (`|GetArrayItem` (`self.Hand_2`))))
    (:`3`
      (return (`|GetArrayItem` (`self.Hand_3`))))))

(fn `ShuffleHand`
  (`|ExecutionSequence`
    (:`then_0`
      (`KismetArrayLibrary.Array_Shuffle` (`self.Hand_0`)))
    (:`then_1`
      (`KismetArrayLibrary.Array_Shuffle` (`self.Hand_1`)))
    (:`then_2`
      (`KismetArrayLibrary.Array_Shuffle` (`self.Hand_2`)))
    (:`then_3`
      (`KismetArrayLibrary.Array_Shuffle` (`self.Hand_3`)))))

(fn `UserConstructionScript`)