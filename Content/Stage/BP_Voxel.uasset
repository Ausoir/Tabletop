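; Voxel world Blueprint for a stage that removes a placed voxel asset actor once the world has loaded.
; BeginPlay runs the parent logic and binds to OnWorldLoaded, whose handler finds a single VoxelAssetActor and destroys it.
; Disconnected experiments remain: one builds boxes from "X" characters in string rows as a grid map, another imports a test data asset at a fixed position.
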(event `self.ReceiveBeginPlay`
  (`parent.ReceiveBeginPlay`)
  (add `self.OnWorldLoaded` (delegate `OnWorldLoaded_Event`)))

(event `OnWorldLoaded_Event`
  (bind _returnvalue (`GameplayStatics.GetActorOfClass` "/Script/Voxel.VoxelAssetActor"))
  (`self.K2_DestroyActor` _returnvalue))

(fn `UserConstructionScript`)